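; Pong game mode that creates the score HUD, tracks player and AI scores, and serves each ball.
; On BeginPlay it picks a random serve direction; each score event updates the HUD and sets the direction for the next serve.
; Serving waits briefly, spawns a new ball, then after another short delay launches it by setting its sphere's physics velocity along X.
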(event EventBeginPlay
  ;[1 1 1] Set references, create widget and set ball speed
  (bind _returnvalue (UserInterface|CreateWidget "/Game/Blueprint/BP_GameHud.BP_GameHud_C"))
  (bind _output_get (Variables|Default|Setm_gameHudRef _returnvalue))
  (UserInterface|Viewport|AddtoViewport _output_get 0)
  (Variables|Default|Setm_direction (Math|Float|Sign(Float) (Math|Random|RandomFloatinRange -1.0 1.0)))
  (Class|PongGameMode|SpawnNewBall))

(event EventSpawnNewBall
  ;[1 1 1] Spawn Ball
  (Utilities|FlowControl|Delay 1.0)
  (bind _returnvalue (Game|SpawnActorfromClass "/Game/Blueprint/BP_Ball.BP_Ball_C" (Math|Transform|MakeTransform "0,10.000000, 0" "0, 0, 0" "1,1,1") "AlwaysSpawn" 0 0))
  (bind _output_get (Variables|Default|Setm_ballRef _returnvalue))
  (Utilities|FlowControl|Delay 0.5)
  (Physics|SetPhysicsLinearVelocity (Variables|/Script/Pong.Ball|Getsphere _output_get) (Math|Vector|MakeVector (* (Variables|Default|Getm_direction) (Variables|Default|Getm_ballSpeed)) 0.0 0.0) false "None"))

(event EventIncreaseAIScore
  ;[1 1 1] Add score functions
  (bind _result (Math|Integer|IncrementInt (Variables|Default|Getm_AIScore))
    (:%20%20
      (Class|GameHud|UpdateAIScore (Variables|Default|Getm_gameHudRef) _result)
      (Variables|Default|Setm_direction -1.0)
      (Class|PongGameMode|SpawnNewBall))))

(event EventIncreasePlayerScore
  ;[1 1 1] Add score functions
  (bind _result (Math|Integer|IncrementInt (Variables|Default|Getm_playerScore))
    (:%20%20
      (Class|GameHud|UpdatePlayerScore (Variables|Default|Getm_gameHudRef) _result)
      (Variables|Default|Setm_direction 1.0)
      (Class|PongGameMode|SpawnNewBall))))

(fn ConstructionScript)